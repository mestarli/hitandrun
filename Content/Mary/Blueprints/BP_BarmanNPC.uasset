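; Barman NPC that patrols three positions and serves drinks by spawning BP_Drink actors.
; A DoOnce on Tick runs a delay-timed loop, using SimpleMoveToLocation to visit middle, end and start positions, then resetting itself.
; At each stop it spawns a drink only if that spot's flag is false, then sets the flag, which this file never clears.
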(event `self.ReceiveBeginPlay`
  ;[1 1 1] Set Start Location of Barman
  (set `self.StartRotation` (`self.K2_GetActorRotation`)))

(event `self.ReceiveTick`
  (params (DeltaSeconds :type "Float (single-precision)"))
  ;[1 1 1] Barman NPC > Servir bebidas
  (`/Engine/EditorBlueprintResources/StandardMacros.DoOnce` false :!label _label
    (:`Completed`
      (`KismetSystemLibrary.Delay` (`self.IntervalWalking`))
      (`AIBlueprintHelperLibrary.SimpleMoveToLocation` (`self.GetController`) (`self.MidlePosition`))
      (`KismetSystemLibrary.Delay` (`self.IntervalWalking`))
      (if (not (`self.MiddleDrink`))
        (`|SpawnActorFromClass` "/Game/Mary/Blueprints/BP_Drink.BP_Drink_C" (`self.SpawnMidleDrink`) "Undefined" "OverrideRootScale" null null)
        (set `self.MiddleDrink` true))
      (`KismetSystemLibrary.Delay` (`self.IntervalWalking`))
      (`AIBlueprintHelperLibrary.SimpleMoveToLocation` (`self.GetController`) (`self.EndPosition`))
      (`KismetSystemLibrary.Delay` (`self.IntervalWalking`))
      (if (not (`self.EndDrink`))
        (`|SpawnActorFromClass` "/Game/Mary/Blueprints/BP_Drink.BP_Drink_C" (`self.SpawnEndDrink`) "Undefined" "OverrideRootScale" null null)
        (set `self.EndDrink` true))
      (`KismetSystemLibrary.Delay` (`self.IntervalWalking`))
      (`AIBlueprintHelperLibrary.SimpleMoveToLocation` (`self.GetController`) (`self.StartPosition`))
      (`KismetSystemLibrary.Delay` (`self.IntervalWalking`))
      (if (not (`self.StartDrink`))
        (`|SpawnActorFromClass` "/Game/Mary/Blueprints/BP_Drink.BP_Drink_C" (`self.SpawnStartDrink`) "Undefined" "OverrideRootScale" null null)
        (set `self.StartDrink` true))
      (`KismetSystemLibrary.Delay` 1.0)
      (goto _label :!via `Reset`))))

(fn `UserConstructionScript`)