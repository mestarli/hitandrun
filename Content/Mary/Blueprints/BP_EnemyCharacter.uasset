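; Enemy character that comes in Fast, Normal and Bigger variants and can chase the player.
; BeginPlay uses NPCType to pick preset enum entries for life, strength and walk speed, converting each entry's name to a number.
; While IsFollowPlayer is set, Tick re-issues a simple move to the player's location every frame.
; The DeleteNPC input only looks up an enemy actor and does nothing with it.
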(event `self.ReceiveBeginPlay`
  ;[1 1 1] Set Variables For diferent type of enemy
  (switch `/Game/Mary/Blueprints/Enemies_Lists/TypeOfNpc` (`self.NPC_Type`)
    (:`NewEnumerator0`
      (bind _output_get (set `self.LifeSelected` "NewEnumerator0"))
      (set `self.Life` (`KismetStringLibrary.Conv_StringToDouble` (`|GetEnumeratorNameAsString` _output_get)))
      (bind _output_get_2 (set `self.StrenghtSelected` "NewEnumerator0"))
      (set `self.Strenght` (`KismetStringLibrary.Conv_StringToDouble` (`|GetEnumeratorNameAsString` _output_get_2)))
      (bind _output_get_3 (set `self.SpeedSelected` "NewEnumerator0"))
      (set `CharacterMovementComponent.MaxWalkSpeed` (`KismetStringLibrary.Conv_StringToDouble` (`|GetEnumeratorNameAsString` _output_get_3)) (`self.CharacterMovement`)))
    (:`NewEnumerator1`
      (bind _output_get_4 (set `self.LifeSelected` "NewEnumerator1"))
      (set `self.Life` (`KismetStringLibrary.Conv_StringToDouble` (`|GetEnumeratorNameAsString` _output_get_4)))
      (bind _output_get_5 (set `self.StrenghtSelected` "NewEnumerator1"))
      (set `self.Strenght` (`KismetStringLibrary.Conv_StringToDouble` (`|GetEnumeratorNameAsString` _output_get_5)))
      (bind _output_get_6 (set `self.SpeedSelected` "NewEnumerator1"))
      (set `CharacterMovementComponent.MaxWalkSpeed` (`KismetStringLibrary.Conv_StringToDouble` (`|GetEnumeratorNameAsString` _output_get_6)) (`self.CharacterMovement`)))
    (:`NewEnumerator2`
      (bind _output_get_7 (set `self.LifeSelected` "NewEnumerator2"))
      (set `self.Life` (`KismetStringLibrary.Conv_StringToDouble` (`|GetEnumeratorNameAsString` _output_get_7)))
      (bind _output_get_8 (set `self.StrenghtSelected` "NewEnumerator2"))
      (set `self.Strenght` (`KismetStringLibrary.Conv_StringToDouble` (`|GetEnumeratorNameAsString` _output_get_8)))
      (bind _output_get_9 (set `self.SpeedSelected` "NewEnumerator2"))
      (set `CharacterMovementComponent.MaxWalkSpeed` (`KismetStringLibrary.Conv_StringToDouble` (`|GetEnumeratorNameAsString` _output_get_9)) (`self.CharacterMovement`)))))

(event `self.ReceiveTick`
  (params (DeltaSeconds :type "Float (single-precision)"))
  ;[1 1 1] Follow Player Logic
  (if (`self.IsFollowPlayer`)
    (`AIBlueprintHelperLibrary.SimpleMoveToLocation` (`self.GetController`) (`self.K2_GetActorLocation` (`GameplayStatics.GetPlayerCharacter` 0)))))

(event `InputAction|DeleteNPC`
  (params (Key :type "Key Structure"))
  (:`Released`
    (`GameplayStatics.GetActorOfClass` "BP_EnemyCharacter_C")))

(fn `UserConstructionScript`)