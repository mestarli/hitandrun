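; BP_Enemy is an enemy character with fast, normal and bigger variants whose type sets life, strength and walk speed.
; BeginPlay sets up physical animation on simulated bodies below a bone, and Tick moves toward the player when following.
; Hard Object_BP impacts subtract their horizontal impulse from life; death makes Tick ragdoll the mesh and disable movement.
; NPC-following, object pickup and gradual-damage test logic are left disconnected.
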(event `self.ReceiveBeginPlay`
  (bind _bonename (`self.BoneName`))
  (bind _physicalanimation (`self.PhysicalAnimation`))
  ;[1 1 1] Ragdoll
  (set `self.EnemyHealth` 5000.0)
  (`PhysicalAnimationComponent.SetSkeletalMeshComponent` _physicalanimation (`self.Mesh`))
  (`PhysicalAnimationComponent.ApplyPhysicalAnimationSettingsBelow` _physicalanimation _bonename (make `PhysicalAnimationData` false 2000.0 10.0 2000.0 10.0) false)
  (`SkeletalMeshComponent.SetAllBodiesBelowSimulatePhysics` (`self.Mesh`) _bonename true false)
  ;[1 1 1] Set Variables For diferent type of enemy
  (switch `/Game/Models/Characters/Enemies/Enemies_Lists/TypeOfNpc` (`self.NPC_Type`)
    (:`NewEnumerator0`
      (bind _output_get (set `self.LifeSelected` "NewEnumerator0"))
      (set `self.Life` (`KismetStringLibrary.Conv_StringToDouble` (`|GetEnumeratorNameAsString` _output_get)))
      (bind _output_get_2 (set `self.StrenghtSelected` "NewEnumerator0"))
      (set `self.Strenght` (`KismetStringLibrary.Conv_StringToDouble` (`|GetEnumeratorNameAsString` _output_get_2)))
      (bind _output_get_3 (set `self.SpeedSelected` "NewEnumerator0"))
      (set `CharacterMovementComponent.MaxWalkSpeed` (`KismetStringLibrary.Conv_StringToDouble` (`|GetEnumeratorNameAsString` _output_get_3)) (`self.CharacterMovement`)))
    (:`NewEnumerator1`
      (bind _output_get_4 (set `self.LifeSelected` "NewEnumerator1"))
      (set `self.Life` (`KismetStringLibrary.Conv_StringToDouble` (`|GetEnumeratorNameAsString` _output_get_4)))
      (bind _output_get_5 (set `self.StrenghtSelected` "NewEnumerator1"))
      (set `self.Strenght` (`KismetStringLibrary.Conv_StringToDouble` (`|GetEnumeratorNameAsString` _output_get_5)))
      (bind _output_get_6 (set `self.SpeedSelected` "NewEnumerator1"))
      (set `CharacterMovementComponent.MaxWalkSpeed` (`KismetStringLibrary.Conv_StringToDouble` (`|GetEnumeratorNameAsString` _output_get_6)) (`self.CharacterMovement`)))
    (:`NewEnumerator2`
      (bind _output_get_7 (set `self.LifeSelected` "NewEnumerator2"))
      (set `self.Life` (`KismetStringLibrary.Conv_StringToDouble` (`|GetEnumeratorNameAsString` _output_get_7)))
      (bind _output_get_8 (set `self.StrenghtSelected` "NewEnumerator2"))
      (set `self.Strenght` (`KismetStringLibrary.Conv_StringToDouble` (`|GetEnumeratorNameAsString` _output_get_8)))
      (bind _output_get_9 (set `self.SpeedSelected` "NewEnumerator2"))
      (set `CharacterMovementComponent.MaxWalkSpeed` (`KismetStringLibrary.Conv_StringToDouble` (`|GetEnumeratorNameAsString` _output_get_9)) (`self.CharacterMovement`)))))

(event `self.ReceiveTick`
  (params (DeltaSeconds :type "Float (single-precision)"))
  (if (`self.Is Dead`)
    (`self.Ragdoll_Death`)
    (else
      ;[1 1 1] Follow Player Logic
      (if (`self.IsFollowPlayer`)
        (`AIBlueprintHelperLibrary.SimpleMoveToLocation` (`self.GetController`) (`self.K2_GetActorLocation` (`GameplayStatics.GetPlayerCharacter` 0)))
        (else
          ;[1 1 1] Follow NPC
          (`/Engine/EditorBlueprintResources/StandardMacros.DoOnce` false))))))

(event `self.Mesh.OnComponentHit`
  (params (HitComponent :type "PrimitiveComponent Object Reference") (OtherActor :type "Actor Object Reference") (OtherComp :type "PrimitiveComponent Object Reference") (NormalImpulse :type "Vector Structure") (Hit :type "HitResult Structure (by ref)"))
  (bind _life (`self.Life`))
  (bind _returnvalue (`KismetMathLibrary.Abs` (`KismetMathLibrary.VSize2D` (`KismetMathLibrary.MakeVector2D` NormalImpulse_X NormalImpulse_Y))))
  (if (not (`self.Is Dead`))
    (cast `/Game/Carlos/Blueprints/Object_BP` OtherActor)
    (if (>= _returnvalue 10000.0)
      (set `self.Life` (- _life _returnvalue))
      (if (> 0.0 _life)
        (set `self.IsDead` true)))))

(fn `EnemyAfterDeath`
  (bind _physicalanimation (`self.PhysicalAnimation`))
  (`PrimitiveComponent.SetSimulatePhysics` (`self.Mesh`) true)
  (`ActorComponent.Deactivate` _physicalanimation)
  (`PhysicalAnimationComponent.ApplyPhysicalAnimationSettingsBelow` _physicalanimation (`self.BoneName`) (make `PhysicalAnimationData` false) false)
  (`SkeletalMeshComponent.Stop` (`self.Mesh`))
  (set `self.IsDead` true))

(fn `Ragdoll_Death`
  ;[1 1 1] Simulate Death
  (`PrimitiveComponent.SetSimulatePhysics` (`self.Mesh`) true)
  (`CharacterMovementComponent.DisableMovement` (`self.CharacterMovement`)))

(fn `UserConstructionScript`)