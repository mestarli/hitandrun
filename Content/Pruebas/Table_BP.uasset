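; Table prop Blueprint that outlines itself through custom depth when the third-person character's MeshDetecter component overlaps its mesh.
; On begin overlap it registers itself as the character's HighlightedItem and enables custom depth, only if no valid item is already highlighted.
; End overlap turns custom depth off but leaves HighlightedItem set.
; The construction script applies the Mesh variable to the StaticMesh component.
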(event `self.StaticMesh.OnComponentBeginOverlap`
  (params (OverlappedComponent :type "PrimitiveComponent Object Reference") (OtherActor :type "Actor Object Reference") (OtherComp :type "PrimitiveComponent Object Reference") (OtherBodyIndex :type Integer) (bFromSweep :type Boolean) (SweepResult :type "HitResult Structure (by ref)"))
  (bind _asbp_third_person_character (cast `/Game/ThirdPerson/Blueprints/BP_ThirdPersonCharacter` OtherActor))
  (if (== OtherComp (`/Game/ThirdPerson/Blueprints/BP_ThirdPersonCharacter.MeshDetecter` _asbp_third_person_character))
    (`/Engine/EditorBlueprintResources/StandardMacros.IsValid` (`/Game/ThirdPerson/Blueprints/BP_ThirdPersonCharacter.Highlighted_Item` _asbp_third_person_character)
      (:`Is Not Valid`
        (set `/Game/ThirdPerson/Blueprints/BP_ThirdPersonCharacter.Highlighted_Item` self _asbp_third_person_character)
        (`PrimitiveComponent.SetRenderCustomDepth` (`self.StaticMesh`) true)))))

(event `self.StaticMesh.OnComponentEndOverlap`
  (params (OverlappedComponent :type "PrimitiveComponent Object Reference") (OtherActor :type "Actor Object Reference") (OtherComp :type "PrimitiveComponent Object Reference") (OtherBodyIndex :type Integer))
  (bind _asbp_third_person_character (cast `/Game/ThirdPerson/Blueprints/BP_ThirdPersonCharacter` OtherActor))
  (if (== OtherComp (`/Game/ThirdPerson/Blueprints/BP_ThirdPersonCharacter.MeshDetecter` _asbp_third_person_character))
    (`PrimitiveComponent.SetRenderCustomDepth` (`self.StaticMesh`) false)))

(fn `UserConstructionScript`
  (`StaticMeshComponent.SetStaticMesh` (`self.StaticMesh`) (`self.Mesh`)))