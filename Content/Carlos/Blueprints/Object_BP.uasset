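; Breakable physics item that the third-person character can highlight, with configurable mass and whole and piece meshes set in the construction script.
; Overlapping the character's MeshDetecter registers it as HighlightedItem, if none is set, and spawns a custom-depth outline mesh.
; While CanHit is set, impacts compare mass times speed against Resistencia.
; Stronger hits swap the mesh for twelve hidden, pre-placed simulated pieces; weaker ones clear CanHit.
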(event `self.ReceiveBeginPlay`
  (`PrimitiveComponent.SetCollisionEnabled` (`self.StaticMesh1`) "NoCollision")
  (`PrimitiveComponent.SetCollisionEnabled` (`self.StaticMesh2`) "NoCollision")
  (`PrimitiveComponent.SetCollisionEnabled` (`self.StaticMesh3`) "NoCollision")
  (`PrimitiveComponent.SetCollisionEnabled` (`self.StaticMesh4`) "NoCollision")
  (`PrimitiveComponent.SetCollisionEnabled` (`self.StaticMesh5`) "NoCollision")
  (`PrimitiveComponent.SetCollisionEnabled` (`self.StaticMesh6`) "NoCollision")
  (`PrimitiveComponent.SetCollisionEnabled` (`self.StaticMesh7`) "NoCollision")
  (`PrimitiveComponent.SetCollisionEnabled` (`self.StaticMesh8`) "NoCollision")
  (`PrimitiveComponent.SetCollisionEnabled` (`self.StaticMesh9`) "NoCollision")
  (`PrimitiveComponent.SetCollisionEnabled` (`self.StaticMesh10`) "NoCollision")
  (`PrimitiveComponent.SetCollisionEnabled` (`self.StaticMesh11`) "NoCollision")
  (`PrimitiveComponent.SetCollisionEnabled` (`self.StaticMesh12`) "NoCollision")
  (`SceneComponent.SetHiddenInGame` (`self.StaticMesh4`) true false)
  (`SceneComponent.SetHiddenInGame` (`self.StaticMesh3`) true false)
  (`SceneComponent.SetHiddenInGame` (`self.StaticMesh2`) true false)
  (`SceneComponent.SetHiddenInGame` (`self.StaticMesh1`) true false)
  (`SceneComponent.SetHiddenInGame` (`self.StaticMesh5`) true false)
  (`SceneComponent.SetHiddenInGame` (`self.StaticMesh6`) true false)
  (`SceneComponent.SetHiddenInGame` (`self.StaticMesh7`) true false)
  (`SceneComponent.SetHiddenInGame` (`self.StaticMesh8`) true false)
  (`SceneComponent.SetHiddenInGame` (`self.StaticMesh9`) true false)
  (`SceneComponent.SetHiddenInGame` (`self.StaticMesh10`) true false)
  (`SceneComponent.SetHiddenInGame` (`self.StaticMesh11`) true false)
  (`SceneComponent.SetHiddenInGame` (`self.StaticMesh12`) true false)
  (`PrimitiveComponent.SetMassOverrideInKg` (`self.StaticMesh`) "None" (`self.ItemMass`) true))

(event `self.StaticMesh.OnComponentBeginOverlap`
  (params (OverlappedComponent :type "PrimitiveComponent Object Reference") (OtherActor :type "Actor Object Reference") (OtherComp :type "PrimitiveComponent Object Reference") (OtherBodyIndex :type Integer) (bFromSweep :type Boolean) (SweepResult :type "HitResult Structure (by ref)"))
  ;[1 1 1] Highlight_Objects
  (bind _asbp_third_person_character (cast `/Game/ThirdPerson/Blueprints/BP_ThirdPersonCharacter` OtherActor))
  (if (== OtherComp (`/Game/ThirdPerson/Blueprints/BP_ThirdPersonCharacter.MeshDetecter` _asbp_third_person_character))
    (`/Engine/EditorBlueprintResources/StandardMacros.IsValid` (`/Game/ThirdPerson/Blueprints/BP_ThirdPersonCharacter.Highlighted_Item` _asbp_third_person_character)
      (:`Is Not Valid`
        (set `/Game/ThirdPerson/Blueprints/BP_ThirdPersonCharacter.Highlighted_Item` self _asbp_third_person_character)
        (bind _returnvalue (`AddComponent|NODE_AddStaticMeshComponent-0`))
        (bind _output_get (set `self.OutlineMesh` _returnvalue))
        (`StaticMeshComponent.SetStaticMesh` _output_get (`self.Mesh`))
        (`PrimitiveComponent.SetRenderCustomDepth` (`self.OutlineMesh`) true)))))

(event `self.StaticMesh.OnComponentEndOverlap`
  (params (OverlappedComponent :type "PrimitiveComponent Object Reference") (OtherActor :type "Actor Object Reference") (OtherComp :type "PrimitiveComponent Object Reference") (OtherBodyIndex :type Integer))
  ;[1 1 1] Highlight_Objects
  (bind _asbp_third_person_character (cast `/Game/ThirdPerson/Blueprints/BP_ThirdPersonCharacter` OtherActor))
  (if (== OtherComp (`/Game/ThirdPerson/Blueprints/BP_ThirdPersonCharacter.MeshDetecter` _asbp_third_person_character))
    (`/Engine/EditorBlueprintResources/StandardMacros.IsValid` (`self.OutlineMesh`)
      (:`Is Valid`
        (set `/Game/ThirdPerson/Blueprints/BP_ThirdPersonCharacter.Highlighted_Item` null _asbp_third_person_character)
        (`ActorComponent.K2_DestroyComponent` (`self.OutlineMesh`))))))

(event `self.StaticMesh.OnComponentHit`
  (params (HitComponent :type "PrimitiveComponent Object Reference") (OtherActor :type "Actor Object Reference") (OtherComp :type "PrimitiveComponent Object Reference") (NormalImpulse :type "Vector Structure") (Hit :type "HitResult Structure (by ref)"))
  (bind _staticmesh1 (`self.StaticMesh1`))
  (bind _returnvalue (/ (* (`KismetMathLibrary.VSize` (`self.GetVelocity`)) (`PrimitiveComponent.GetMass` (`self.StaticMesh`))) 1000.0))
  (if (`self.CanHit`)
    (`KismetSystemLibrary.PrintString` (`KismetStringLibrary.Conv_DoubleToString` _returnvalue))
    (if (> _returnvalue (`self.Resistencia`))
      (`ActorComponent.K2_DestroyComponent` (`self.StaticMesh`))
      (`SceneComponent.SetHiddenInGame` _staticmesh1 false false)
      (`SceneComponent.SetHiddenInGame` (`self.StaticMesh2`) false false)
      (`SceneComponent.SetHiddenInGame` (`self.StaticMesh3`) false false)
      (`SceneComponent.SetHiddenInGame` (`self.StaticMesh4`) false false)
      (`SceneComponent.SetHiddenInGame` (`self.StaticMesh5`) false false)
      (`SceneComponent.SetHiddenInGame` (`self.StaticMesh6`) false false)
      (`SceneComponent.SetHiddenInGame` (`self.StaticMesh7`) false false)
      (`SceneComponent.SetHiddenInGame` (`self.StaticMesh8`) false false)
      (`SceneComponent.SetHiddenInGame` (`self.StaticMesh9`) false false)
      (`SceneComponent.SetHiddenInGame` (`self.StaticMesh10`) false false)
      (`SceneComponent.SetHiddenInGame` (`self.StaticMesh11`) false false)
      (`SceneComponent.SetHiddenInGame` (`self.StaticMesh12`) false false)
      (`PrimitiveComponent.SetCollisionEnabled` _staticmesh1 "QueryAndPhysics")
      (`PrimitiveComponent.SetCollisionEnabled` (`self.StaticMesh2`) "QueryAndPhysics")
      (`PrimitiveComponent.SetCollisionEnabled` (`self.StaticMesh3`) "QueryAndPhysics")
      (`PrimitiveComponent.SetCollisionEnabled` (`self.StaticMesh4`) "QueryAndPhysics")
      (`PrimitiveComponent.SetCollisionEnabled` (`self.StaticMesh5`) "QueryAndPhysics")
      (`PrimitiveComponent.SetCollisionEnabled` (`self.StaticMesh6`) "QueryAndPhysics")
      (`PrimitiveComponent.SetCollisionEnabled` (`self.StaticMesh7`) "QueryAndPhysics")
      (`PrimitiveComponent.SetCollisionEnabled` (`self.StaticMesh8`) "QueryAndPhysics")
      (`PrimitiveComponent.SetCollisionEnabled` (`self.StaticMesh9`) "QueryAndPhysics")
      (`PrimitiveComponent.SetCollisionEnabled` (`self.StaticMesh10`) "QueryAndPhysics")
      (`PrimitiveComponent.SetCollisionEnabled` (`self.StaticMesh11`) "QueryAndPhysics")
      (`PrimitiveComponent.SetCollisionEnabled` (`self.StaticMesh12`) "QueryAndPhysics")
      (`PrimitiveComponent.SetSimulatePhysics` _staticmesh1 true)
      (`PrimitiveComponent.SetSimulatePhysics` (`self.StaticMesh2`) true)
      (`PrimitiveComponent.SetSimulatePhysics` (`self.StaticMesh3`) true)
      (`PrimitiveComponent.SetSimulatePhysics` (`self.StaticMesh4`) true)
      (`PrimitiveComponent.SetSimulatePhysics` (`self.StaticMesh5`) true)
      (`PrimitiveComponent.SetSimulatePhysics` (`self.StaticMesh6`) true)
      (`PrimitiveComponent.SetSimulatePhysics` (`self.StaticMesh7`) true)
      (`PrimitiveComponent.SetSimulatePhysics` (`self.StaticMesh8`) true)
      (`PrimitiveComponent.SetSimulatePhysics` (`self.StaticMesh9`) true)
      (`PrimitiveComponent.SetSimulatePhysics` (`self.StaticMesh10`) true)
      (`PrimitiveComponent.SetSimulatePhysics` (`self.StaticMesh11`) true)
      (`PrimitiveComponent.SetSimulatePhysics` (`self.StaticMesh12`) true)
      (else
        (set `self.CanHit` false)))))

(fn `UserConstructionScript`
  (`StaticMeshComponent.SetStaticMesh` (`self.StaticMesh`) (`self.Mesh`))
  (`StaticMeshComponent.SetStaticMesh` (`self.StaticMesh1`) (`self.Mesh_1`))
  (`StaticMeshComponent.SetStaticMesh` (`self.StaticMesh2`) (`self.Mesh_2`))
  (`StaticMeshComponent.SetStaticMesh` (`self.StaticMesh3`) (`self.Mesh_3`))
  (`StaticMeshComponent.SetStaticMesh` (`self.StaticMesh4`) (`self.Mesh_4`))
  (`StaticMeshComponent.SetStaticMesh` (`self.StaticMesh5`) (`self.Mesh_5`))
  (`StaticMeshComponent.SetStaticMesh` (`self.StaticMesh6`) (`self.Mesh_6`))
  (`StaticMeshComponent.SetStaticMesh` (`self.StaticMesh7`) (`self.Mesh_7`))
  (`StaticMeshComponent.SetStaticMesh` (`self.StaticMesh8`) (`self.Mesh_8`))
  (`StaticMeshComponent.SetStaticMesh` (`self.StaticMesh9`) (`self.Mesh_9`))
  (`StaticMeshComponent.SetStaticMesh` (`self.StaticMesh10`) (`self.Mesh_10`))
  (`StaticMeshComponent.SetStaticMesh` (`self.StaticMesh11`) (`self.Mesh_11`))
  (`StaticMeshComponent.SetStaticMesh` (`self.StaticMesh12`) (`self.Mesh_12`)))