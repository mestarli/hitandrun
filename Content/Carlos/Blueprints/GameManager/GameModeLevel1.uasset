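; Level 1 game mode that tracks object destruction and opens the Teteria level when progress reaches 100%.
; BeginPlay sets the target to half the Object_BP count, gated by a strength check between the player and the loop's array element.
; Tick polls every object, clears broken flags and adds normalized progress.
; Each break also switches enemies from following NPCs to chasing the player until a follower cap is reached.
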(event `self.ReceiveBeginPlay`
  (bind _asbp_third_person_character (cast `/Game/ThirdPerson/Blueprints/BP_ThirdPersonCharacter` (`GameplayStatics.GetPlayerCharacter` 0)))
  (bind _outactors (`GameplayStatics.GetAllActorsOfClass` "/Game/Carlos/Blueprints/Object_BP.Object_BP_C"))
  (for _array_element _outactors
    _)
  (if (<= (`/Game/Carlos/Blueprints/Object_BP.FuerzaParaRecojer` _array_element) (`/Game/ThirdPerson/Blueprints/BP_ThirdPersonCharacter.Fuerza` _asbp_third_person_character))
    (set `self.NumberObjects` (/ (`KismetArrayLibrary.Array_Length` _outactors) 2))))

(event `self.ReceiveTick`
  (params (DeltaSeconds :type "Float (single-precision)"))
  (`|ExecutionSequence`
    (:`then_0`
      (bind _outactors (`GameplayStatics.GetAllActorsOfClass` "/Game/Carlos/Blueprints/Object_BP.Object_BP_C"))
      (for _array_element _outactors
        (if (`/Game/Carlos/Blueprints/Object_BP.IsBreaked` _array_element)
          (set `/Game/Carlos/Blueprints/Object_BP.IsBreaked` false _array_element)
          (bind _output_get (set `self.ObjectsBreaked` (+ (stale _output_get) (/ (/ 100 (`self.NumberObjects`)) 100))))
          (if (>= (`self.ObjectsBreaked`) 0.0)
            (bind _outactors_2 (`GameplayStatics.GetAllActorsOfClass` "/Game/Models/Characters/Enemies/BP_EnemyCharacter.BP_EnemyCharacter_C"))
            (for _array_element_2 _outactors_2
              (if (not (>= (`self.EnemiesFollowPlayer`) (`self.MaxFollowEnem`)))
                (set `/Game/Models/Characters/Enemies/BP_EnemyCharacter.IsFollowPlayer` true _array_element_2)
                (`/Engine/EditorBlueprintResources/StandardMacros.IncrementInt` (`self.EnemiesFollowPlayer`)
                  (:`  `
                    (set `/Game/Models/Characters/Enemies/BP_EnemyCharacter.IsFollowNPC` false _array_element_2)))))))))
    (:`then_1`
      (if (>= (`self.ObjectsBreaked`) 1.0)
        (`GameplayStatics.OpenLevel` "Teteria")))))

(fn `UserConstructionScript`)