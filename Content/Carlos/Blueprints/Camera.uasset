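; Camera actor that shadows the third-person player and aims at their follow camera once they die.
; On BeginPlay it caches the player character, then each Tick does a swept move to the player's X and Y at double the player's world Z.
; While IsDeath is set, it activates its camera component and rotates it every Tick toward the player's FollowCamera using a look-at rotation.
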(event `self.ReceiveBeginPlay`
  (bind _asbp_third_person_character (cast `/Game/ThirdPerson/Blueprints/BP_ThirdPersonCharacter` (`GameplayStatics.GetPlayerCharacter` 0)))
  (set `self.ThirdPersonPlayer` _asbp_third_person_character))

(event `self.ReceiveTick`
  (params (DeltaSeconds :type "Float (single-precision)"))
  (bind _thirdpersonplayer (`self.ThirdPersonPlayer`))
  (bind _camera (`self.Camera`))
  (bind (_returnvalue_x _returnvalue_y _returnvalue_z) (`KismetMathLibrary.BreakVector` (`self.K2_GetActorLocation` _thirdpersonplayer)))
  (`self.K2_SetActorLocation` (`KismetMathLibrary.MakeVector` _returnvalue_x _returnvalue_y (* _returnvalue_z 2.0)) true)
  (if (`/Game/ThirdPerson/Blueprints/BP_ThirdPersonCharacter.IsDeath` _thirdpersonplayer)
    (`ActorComponent.Activate` _camera false)
    (`SceneComponent.K2_SetWorldRotation` _camera (`KismetMathLibrary.FindLookAtRotation` (`self.K2_GetActorLocation`) (`SceneComponent.K2_GetComponentLocation` (`/Game/ThirdPerson/Blueprints/BP_ThirdPersonCharacter.FollowCamera` _thirdpersonplayer))) false false)))

(fn `UserConstructionScript`)