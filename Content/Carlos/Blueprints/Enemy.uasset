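; Enemy that gives a physics-driven body reaction when its capsule begins overlapping a Table_BP.
; BeginPlay sets up physical animation and simulation from the Hips down.
; The overlap sets full physics blend weight on bones below Hips and starts a short timer.
; That timer flip-flops a flag that lets Tick interpolate the weight back down, then a second timer clears the flag and resets the state.
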(event `self.ReceiveBeginPlay`
  (`PhysicalAnimationComponent.SetSkeletalMeshComponent` (`self.PhysicalAnimation`) (`self.Mesh`))
  (`PhysicalAnimationComponent.ApplyPhysicalAnimationSettingsBelow` (`self.PhysicalAnimation`) (`self.Hips`) (make `PhysicalAnimationData` false 500.0 100.0 500.0 100.0) true)
  (`SkeletalMeshComponent.SetAllBodiesBelowSimulatePhysics` (`self.Mesh`) (`self.Hips`) true true)
  (`SkeletalMeshComponent.SetAllBodiesBelowPhysicsBlendWeight` (`self.Mesh`) (`self.Hips`) 0.0 false false))

(event `self.ReceiveTick`
  (params (DeltaSeconds :type "Float (single-precision)"))
  (if (`self.DisablePA`)
    (`self.SlowlyDisablePA`)
    (`/Engine/EditorBlueprintResources/StandardMacros.DoOnce` false :!label _label
      (:`Completed`
        (`KismetSystemLibrary.K2_SetTimer` null "DisablePhysicalAnimation" 0.2)))))

(event `DisablePhysicalAnimation`
  (`/Engine/EditorBlueprintResources/StandardMacros.FlipFlop`
    (:`A`
      (set `self.DisablePA` true))
    (:`B`
      (set `self.DisablePA` false)
      (set `self.Current` 1.0)
      (goto _label :!via `Reset`))))

(event `self.CapsuleComponent.OnComponentBeginOverlap`
  (params (OverlappedComponent :type "PrimitiveComponent Object Reference") (OtherActor :type "Actor Object Reference") (OtherComp :type "PrimitiveComponent Object Reference") (OtherBodyIndex :type Integer) (bFromSweep :type Boolean) (SweepResult :type "HitResult Structure (by ref)"))
  (cast `/Game/Carlos/Blueprints/Table_BP` OtherActor)
  (`SkeletalMeshComponent.SetAllBodiesBelowPhysicsBlendWeight` (`self.Mesh`) (`self.Hips`) 1.0 false false)
  (`KismetSystemLibrary.K2_SetTimer` null "DisablePhysicalAnimation" 0.2))

(event `SlowlyDisablePA`
  (bind _output_get (set `self.Current` (`KismetMathLibrary.FInterpTo` (`self.Current`) 0.0 (`GameplayStatics.GetWorldDeltaSeconds`) 10.0)))
  (`SkeletalMeshComponent.SetAllBodiesBelowPhysicsBlendWeight` (`self.Mesh`) (`self.Hips`) _output_get false false))

(fn `UserConstructionScript`)