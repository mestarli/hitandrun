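; Table Blueprint actor with a configurable mesh that highlights when the third-person character's MeshDetecter component overlaps it.
; The construction script applies Mesh to StaticMesh.
; On overlap, if the character has no HighlightedItem, it registers itself there and spawns a duplicate mesh component rendering to custom depth.
; When overlap ends with a valid outline mesh, it clears that reference and destroys the duplicate.
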(event `self.StaticMesh.OnComponentBeginOverlap`
  (params (OverlappedComponent :type "PrimitiveComponent Object Reference") (OtherActor :type "Actor Object Reference") (OtherComp :type "PrimitiveComponent Object Reference") (OtherBodyIndex :type Integer) (bFromSweep :type Boolean) (SweepResult :type "HitResult Structure (by ref)"))
  ;[1 1 1] Highlight_Objects
  (bind _asbp_third_person_character (cast `/Game/ThirdPerson/Blueprints/BP_ThirdPersonCharacter` OtherActor))
  (if (== OtherComp (`/Game/ThirdPerson/Blueprints/BP_ThirdPersonCharacter.MeshDetecter` _asbp_third_person_character))
    (`/Engine/EditorBlueprintResources/StandardMacros.IsValid` (`/Game/ThirdPerson/Blueprints/BP_ThirdPersonCharacter.Highlighted_Item` _asbp_third_person_character)
      (:`Is Not Valid`
        (set `/Game/ThirdPerson/Blueprints/BP_ThirdPersonCharacter.Highlighted_Item` self _asbp_third_person_character)
        (bind _returnvalue (`AddComponent|NODE_AddStaticMeshComponent-0`))
        (bind _output_get (set `self.OutlineMesh` _returnvalue))
        (`StaticMeshComponent.SetStaticMesh` _output_get (`self.Mesh`))
        (`PrimitiveComponent.SetRenderCustomDepth` (`self.OutlineMesh`) true)))))

(event `self.StaticMesh.OnComponentEndOverlap`
  (params (OverlappedComponent :type "PrimitiveComponent Object Reference") (OtherActor :type "Actor Object Reference") (OtherComp :type "PrimitiveComponent Object Reference") (OtherBodyIndex :type Integer))
  ;[1 1 1] Highlight_Objects
  (bind _asbp_third_person_character (cast `/Game/ThirdPerson/Blueprints/BP_ThirdPersonCharacter` OtherActor))
  (if (== OtherComp (`/Game/ThirdPerson/Blueprints/BP_ThirdPersonCharacter.MeshDetecter` _asbp_third_person_character))
    (`/Engine/EditorBlueprintResources/StandardMacros.IsValid` (`self.OutlineMesh`)
      (:`Is Valid`
        (set `/Game/ThirdPerson/Blueprints/BP_ThirdPersonCharacter.Highlighted_Item` null _asbp_third_person_character)
        (`ActorComponent.K2_DestroyComponent` (`self.OutlineMesh`))))))

(fn `UserConstructionScript`
  (`StaticMeshComponent.SetStaticMesh` (`self.StaticMesh`) (`self.Mesh`)))